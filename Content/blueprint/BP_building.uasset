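; BP_building is a defensive turret that finds BP_Enemy pawns in range and fires bullets at them.
; CheckEnemies, run by a looping timer or by Tick when targetless, sphere-traces for enemies, picks one at random and stops the timer.
; Tick yaws the Cylinder toward the target, using a Delay to pace BP_Bullet spawns from the Gun with that target passed in.
; Targets leaving range are dropped and the search timer restarts.
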(event `recheck`
  (bind _returnvalue (`KismetSystemLibrary.K2_SetTimerDelegate` (delegate `check enemies`) 0.5 true :!label _label))
  (set `self.set enemy` _returnvalue))

(event `self.ReceiveBeginPlay`
  (goto _label))

(event `check enemies`
  (bind _returnvalue (`self.K2_GetActorLocation`))
  (bind _enemy_array (`self.enemy_array`))
  (`KismetArrayLibrary.Array_Clear` (`self.enemy_array`))
  (bind _outhits (`KismetSystemLibrary.SphereTraceMultiForObjects` _returnvalue _returnvalue 1000.0 (`|MakeArray` "ObjectTypeQuery3" :!type "EObjectTypeQuery Enum")))
  (for _array_element _outhits
    (bind _asbp_enemy (cast `/Game/ThirdPersonBP/Blueprints/BP_Enemy` (`.HitActor` (`GameplayStatics.BreakHitResult` _array_element))))
    (`KismetArrayLibrary.Array_Add` (`self.enemy_array`) _asbp_enemy))
  (if (not (== (`KismetArrayLibrary.Array_Length` (`self.enemy_array`)) 0))
    (set `self.target` (`|GetArrayItem` _enemy_array (`KismetMathLibrary.RandomIntegerInRange` 0 (- (`KismetArrayLibrary.Array_Length` _enemy_array) 1))))
    (`KismetSystemLibrary.K2_ClearAndInvalidateTimerHandle` (`self.set enemy`))))

(event `self.ReceiveTick`
  (params (DeltaSeconds :type "Float (single-precision)"))
  (bind (_returnvalue_roll _returnvalue_pitch _returnvalue_yaw) (`KismetMathLibrary.BreakRotator` (`KismetMathLibrary.FindLookAtRotation` (`SceneComponent.K2_GetComponentLocation` (`self.Cylinder`)) (`self.K2_GetActorLocation` (`self.target`)))))
  (`self.target`
    (:`then`
      (`SceneComponent.K2_SetWorldRotation` (`self.Cylinder`) (`KismetMathLibrary.MakeRotator` 0.0 0.0 _returnvalue_yaw) false false)
      (if (>= (`KismetMathLibrary.VSize` (- (`SceneComponent.K2_GetComponentLocation` (`self.Cylinder`)) (`self.K2_GetActorLocation` (`self.target`)))) 1000.0)
        (set `self.target` null)
        (`self.recheck`)
        (else
          (`KismetSystemLibrary.Delay` 0.5)
          (bind _target (`self.target`)
            (:`then`
              (`|SpawnActorFromClass` "/Game/blueprint/BP_Bullet.BP_Bullet_C" (`KismetMathLibrary.MakeTransform` (`SceneComponent.K2_GetComponentLocation` (`self.gun`)) (`KismetMathLibrary.MakeRotator` 0.0 (.pitch (.rotation (`self.GetTransform`))))) "Undefined" "OverrideRootScale" null _target null))
            (:`else`)))))
    (:`else`
      (`self.check enemies`))))

(fn `UserConstructionScript`)