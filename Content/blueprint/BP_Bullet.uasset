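; BP_Bullet is a homing projectile that chases a target actor and damages enemies it touches.
; Each tick, while TargetType is valid, it computes the look-at direction to the target and feeds it, at fixed speed, to ProjectileMovement as a local-space velocity.
; When its Box overlaps any BP_Enemy, not only the target, it calls TakeDamage with a fixed amount and destroys itself.
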(event `self.ReceiveTick`
  (params (DeltaSeconds :type "Float (single-precision)"))
  (bind _target_type (`self.target_type`)
    (:`then`
      (`ProjectileMovementComponent.SetVelocityInLocalSpace` (`self.ProjectileMovement`) (* (`KismetMathLibrary.Conv_RotatorToVector` (`KismetMathLibrary.FindLookAtRotation` (`self.K2_GetActorLocation`) (`self.K2_GetActorLocation` _target_type))) 1500.0)))
    (:`else`)))

(event `self.Box.OnComponentBeginOverlap`
  (params (OverlappedComponent :type "PrimitiveComponent Object Reference") (OtherActor :type "Actor Object Reference") (OtherComp :type "PrimitiveComponent Object Reference") (OtherBodyIndex :type Integer) (bFromSweep :type Boolean) (SweepResult :type "HitResult Structure (by ref)"))
  (bind _asbp_enemy (cast `/Game/ThirdPersonBP/Blueprints/BP_Enemy` OtherActor))
  (`/Game/ThirdPersonBP/Blueprints/BP_Enemy.TakeDamage` _asbp_enemy 10.0)
  (`self.K2_DestroyActor`))

(fn `UserConstructionScript`)