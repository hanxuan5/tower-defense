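; Bullet projectile that homes in on a target actor and damages enemies.
; Each tick it computes the look-at direction to its TargetType actor and passes it, scaled to a fixed speed, to the ProjectileMovement component as local-space velocity.
; When its Box component overlaps a BP_Enemy, it applies fixed damage and destroys itself, ignoring other actors.
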(event `self.ReceiveTick`
  (params (DeltaSeconds :type "Float (single-precision)"))
  (`ProjectileMovementComponent.SetVelocityInLocalSpace` (`self.ProjectileMovement`) (* (`KismetMathLibrary.Conv_RotatorToVector` (`KismetMathLibrary.FindLookAtRotation` (`self.K2_GetActorLocation`) (`self.K2_GetActorLocation` (`self.target_type`)))) 600.0)))

(event `self.Box.OnComponentBeginOverlap`
  (params (OverlappedComponent :type "PrimitiveComponent Object Reference") (OtherActor :type "Actor Object Reference") (OtherComp :type "PrimitiveComponent Object Reference") (OtherBodyIndex :type Integer) (bFromSweep :type Boolean) (SweepResult :type "HitResult Structure (by ref)"))
  (bind _asbp_enemy (cast `/Game/blueprint/BP_Enemy` OtherActor))
  (`GameplayStatics.ApplyDamage` _asbp_enemy 10.0)
  (`self.K2_DestroyActor`))

(fn `UserConstructionScript`)