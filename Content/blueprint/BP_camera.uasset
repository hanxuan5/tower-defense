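; Camera Blueprint for drag-and-drop placement of buildings with the mouse, which also creates the W_hud widget.
; DragMesh spawns a BP_Building at the traced cursor point, ignoring its Index, and starts dragging.
; Tick moves it in X and Y along a Visibility trace toward the deprojected mouse direction, falling back to the ray's end.
; Releasing the left button drops it and enables collision, though the disable-collision node is unconnected.
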(event `Key|LeftMouseButton`
  (params (Key :type "Key Structure"))
  (:`Released`
    (`KismetSystemLibrary.PrintString` "release")
    (set `self.CanDrag` false)
    (`self.SetActorEnableCollision` (`self.CurrentControlActor`) true)
    (set `self.CurrentControlActor` null)))

(event `self.ReceiveBeginPlay`
  (bind _returnvalue (`GameplayStatics.GetPlayerController` 0))
  (bind _returnvalue_2 (`|CreateWidget` "/Game/widget/W_hud.W_hud_C" null (`self.Mesh`)))
  (`UserWidget.AddToViewport` _returnvalue_2 0)
  (`WidgetBlueprintLibrary.SetInputMode_GameAndUIEx` _returnvalue _returnvalue_2)
  (set `PlayerController.bShowMouseCursor` true _returnvalue))

(event `self.ReceiveTick`
  (params (DeltaSeconds :type "Float (single-precision)"))
  (bind _returnvalue (+ (* (`.WorldDirection` (`PlayerController.DeprojectMousePositionToWorld` (`GameplayStatics.GetPlayerController` 0))) 1000.0) (`self.K2_GetActorLocation`)))
  (if (`self.CanDrag`)
    (`/Engine/EditorBlueprintResources/StandardMacros.IsValid` (`self.CurrentControlActor`)
      (:`Is Valid`
        (bind (_outhit _returnvalue_2) (`KismetSystemLibrary.LineTraceSingle` :`Start` (`self.K2_GetActorLocation`) :`End` _returnvalue :`TraceChannel` "TraceTypeQuery1" :`DrawDebugType` "ForDuration"))
        (bind (_returnvalue_x _returnvalue_y) (`KismetMathLibrary.BreakVector` (`KismetMathLibrary.SelectVector` (`.Location` (`GameplayStatics.BreakHitResult` _outhit)) _returnvalue _returnvalue_2)))
        (`self.K2_SetActorLocation` (`self.CurrentControlActor`) (`KismetMathLibrary.MakeVector` _returnvalue_x _returnvalue_y) false false)))))

(event `DragMesh`
  (params (index :type Integer))
  (bind _returnvalue (+ (* (`.WorldDirection` (`PlayerController.DeprojectMousePositionToWorld` (`GameplayStatics.GetPlayerController` 0))) 1000.0) (`self.K2_GetActorLocation`)))
  (`KismetSystemLibrary.PrintString` "press")
  (bind (_outhit _returnvalue_2) (`KismetSystemLibrary.LineTraceSingle` :`Start` (`self.K2_GetActorLocation`) :`End` _returnvalue :`TraceChannel` "TraceTypeQuery1" :`DrawDebugType` "ForDuration"))
  (bind _returnvalue_3 (`|SpawnActorFromClass` "/Game/blueprint/BP_building.BP_Building_C" (`KismetMathLibrary.MakeTransform` (`KismetMathLibrary.SelectVector` (`.Location` (`GameplayStatics.BreakHitResult` _outhit)) _returnvalue _returnvalue_2)) "Undefined" "OverrideRootScale" null null))
  (set `self.CurrentControlActor` _returnvalue_3)
  (set `self.CanDrag` true))

(fn `UserConstructionScript`)