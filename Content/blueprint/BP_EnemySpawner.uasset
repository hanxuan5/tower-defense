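; Spawner actor that endlessly creates BP_Enemy actors along the edges of a square area centered on the world origin.
; BeginPlay loops SpawnEnemy with a Delay node, using random edge positions, cardinal yaws and slightly varied scale.
; Tick gradually shrinks the Delay variable toward a floor, so spawns speed up over time.
; SetDelay restores a longer interval but is not called within this Blueprint.
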(event `self.ReceiveBeginPlay`
  (`self.SpawnEnemy` :!label _label)
  (`KismetSystemLibrary.Delay` (`self.Delay`))
  (goto _label))

(event `self.ReceiveTick`
  (params (DeltaSeconds :type "Float (single-precision)"))
  (if (> (`self.Delay`) 3.0)
    (set `self.Delay` (- (`self.Delay`) (/ DeltaSeconds 20.0)))))

(fn `SetDelay`
  (set `self.Delay` 12.0))

(fn `SpawnEnemy`
  (bind _returnvalue (`KismetMathLibrary.RandomIntegerInRange` 0 3))
  (bind _returnvalue_2 (`KismetMathLibrary.RandomFloatInRange` 0.8 1.2))
  (bind _returnvalue_3 (`KismetMathLibrary.RandomFloatInRange` -2000.0 2000.0))
  (`|SpawnActorFromClass` "/Game/ThirdPersonBP/Blueprints/BP_Enemy.BP_Enemy_C" (`KismetMathLibrary.MakeTransform` (select `int` _returnvalue :`0` (`KismetMathLibrary.MakeVector` -2000.0 _returnvalue_3) :`1` (`KismetMathLibrary.MakeVector` 2000.0 _returnvalue_3) :`2` (`KismetMathLibrary.MakeVector` _returnvalue_3 -2000.0) :`3` (`KismetMathLibrary.MakeVector` _returnvalue_3 2000.0) :!type "Vector Structure") (`KismetMathLibrary.MakeRotator` 0.0 0.0 (select `int` _returnvalue :`0` 0.0 :`1` 180.0 :`2` 90.0 :`3` 270.0 :!type "Float (single-precision)")) (`KismetMathLibrary.MakeVector` _returnvalue_2 _returnvalue_2 _returnvalue_2)) "Undefined" "OverrideRootScale" null null))

(fn `UserConstructionScript`)